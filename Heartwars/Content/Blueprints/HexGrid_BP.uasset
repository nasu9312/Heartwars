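; HexGrid_BP is an actor Blueprint that lays out a hex-style grid of static mesh components in its construction script.
; Nested loops over GridX and GridY add one mesh component per cell, positioned by SpacingX and SpacingY.
; Odd X columns shift along Y by Offset, creating the staggered hex pattern.
; The event graph holds only disabled placeholder events, so the actor has no runtime logic.
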(fn `UserConstructionScript`
  (bind _index (`/Engine/EditorBlueprintResources/StandardMacros.ForLoopAlt` 0 (`self.gridX`))
    (:`Loop Body`
      (bind _index_2 (`/Engine/EditorBlueprintResources/StandardMacros.ForLoopAlt` 0 (`self.gridY`))
        (:`Loop Body`
          (bind _returnvalue (* _index (`self.spacingX`)))
          (bind _returnvalue_2 (* _index_2 (`self.spacingY`)))
          (`AddComponent|NODE_AddStaticMeshComponent-0` :`RelativeTransform` (`KismetMathLibrary.MakeTransform` (`KismetMathLibrary.SelectVector` (`KismetMathLibrary.MakeVector` _returnvalue _returnvalue_2) (`KismetMathLibrary.MakeVector` _returnvalue (+ _returnvalue_2 (`self.offset`))) (== (mod _index 2) 0)))))))))